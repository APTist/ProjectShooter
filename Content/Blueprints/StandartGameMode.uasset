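; StandartGameMode is a game mode that starts enemy spawning and handles player respawning.
; On BeginPlay it finds the first EnemySpawner in the level and runs its SpawnEnemy function on a looping timer, paced by SpawnEnemyPerSecond.
; The RespawnPlayer event spawns a new HeroCharacter at PlayerSpawnTransform and has player controller 0 possess it.
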(event `self.ReceiveBeginPlay`
  (bind _outactors (`GameplayStatics.GetAllActorsOfClass` "/Game/Blueprints/EnemySpawner.EnemySpawner_C"))
  (bind _output_get (set `self.Spawner` (`|GetArrayItem` _outactors)))
  (`KismetSystemLibrary.K2_SetTimer` _output_get "SpawnEnemy" (/ 1.0 (`self.SpawnEnemyPerSecond`)) true))

(event `Respawn Player`
  (bind _returnvalue (`|SpawnActorFromClass` "/Game/Blueprints/HeroCharacter.HeroCharacter_C" (`self.PlayerSpawnTransform`) "Undefined" "OverrideRootScale" null null))
  (`Controller.Possess` (`GameplayStatics.GetPlayerController` 0) _returnvalue))

(fn `UserConstructionScript`)