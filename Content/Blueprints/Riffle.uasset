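; Rifle Blueprint that fires projectiles automatically while the trigger is held.
; PullTrigger passes a DoOnce gate, fires immediately, then starts a looping timer on Fire at an interval derived from the ShootInSecond rate.
; Fire spawns the Projectile class at the ProjectileSwapner component's world transform.
; ReleaseTrigger clears the timer and resets the gate.
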(event `PullTrigger`
  (`/Engine/EditorBlueprintResources/StandardMacros.DoOnce` false :!label _label
    (:`Completed`
      (`self.Fire`)
      (`KismetSystemLibrary.K2_SetTimer` null "Fire" (/ 1.0 (`self.ShootInSecond`)) true))))

(event `ReleaseTrigger`
  (`KismetSystemLibrary.K2_ClearTimer` null "Fire")
  (goto _label :!via `Reset`))

(event `Fire`
  (`|SpawnActorFromClass` "/Game/Blueprints/Projectile.Projectile_C" (`SceneComponent.K2_GetComponentToWorld` (`self.ProjectileSwapner`)) "Undefined" "OverrideRootScale" null null))

(fn `UserConstructionScript`)