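; Enemy character that deals repeating damage to an overlapping hero and can itself be killed.
; Overlap with a HeroCharacter starts a looping timer at AttacksPerSecond that calls the player's AffectHealth, cleared when that player leaves.
; On death it ignores Pawn and WorldDynamic collisions, destroys its DamageVolume, increments the game mode's score, detaches its controller and despawns after a delay.
; The construction script tints a dynamic body material with EnemyColor.
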(event `/Game/Blueprints/I_Damagable.AffectHealth`
  (params (Delta :type "Float (single-precision)"))
  (bind _capsulecomponent (`self.CapsuleComponent`))
  (`self.CalculateHealth` Delta)
  (if (`self.isDead`)
    (`PrimitiveComponent.SetCollisionResponseToChannel` _capsulecomponent "ECC_WorldDynamic" "ECR_Ignore")
    (`PrimitiveComponent.SetCollisionResponseToChannel` _capsulecomponent "ECC_Pawn" "ECR_Ignore")
    (`ActorComponent.K2_DestroyComponent` (`self.DamageVolume`))
    (bind _asstandart_game_mode (cast `/Game/Blueprints/StandartGameMode` (`GameplayStatics.GetGameMode`)))
    (`/Game/Blueprints/StandartGameMode.Increment Score` _asstandart_game_mode 1)
    (`self.DetachFromControllerPendingDestroy`)
    (`KismetSystemLibrary.Delay` 3.0)
    (`self.K2_DestroyActor`)))

(event `self.ReceiveActorBeginOverlap`
  (params (OtherActor :type "Actor Object Reference"))
  (bind _ashero_character (cast `/Game/Blueprints/HeroCharacter` OtherActor))
  (set `self.Player` _ashero_character)
  (`KismetSystemLibrary.K2_SetTimer` null "DamageThePlayer" (/ 1.0 (`self.AttacksPerSecond`)) true))

(event `self.ReceiveActorEndOverlap`
  (params (OtherActor :type "Actor Object Reference"))
  (if (== OtherActor (`self.Player`))
    (`KismetSystemLibrary.K2_ClearTimer` null "DamageThePlayer")))

(event `DamageThePlayer`
  (`/Game/Blueprints/HeroCharacter.AffectHealth` (`self.Player`) (`self.Damage`)))

(fn `UserConstructionScript`
  ;[1 1 1] ChangeMaterialInst
  (bind _returnvalue (`PrimitiveComponent.CreateDynamicMaterialInstance` (`self.Mesh`) 0 null "None"))
  (bind _output_get (set `self.DynamicMat` _returnvalue))
  (`MaterialInstanceDynamic.SetVectorParameterValue` _output_get "BodyColor" (`self.EnemyColor`)))